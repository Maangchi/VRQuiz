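; Media player Blueprint that streams video from URLs, starting with a hardcoded Google Drive API link on BeginPlay.
; PlayVideoFromURL writes the address to a stream media source, opens it on the media player and binds the media sound to that player.
; The ChangeVideo event repeats the same steps inline to switch to a supplied URL.
; The Delay after the initial playback call leads to no further logic.
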(event EventChangeVideo
  (params (URL :type String))
  (Variables|/Script/MediaAssets.StreamMediaSource|SetStreamUrl (Variables|Default|GetStreamMediaSource) URL)
  (Media|MediaPlayer|OpenSource (Variables|Default|GetMedia%20Player) (Variables|Default|GetStreamMediaSource))
  (Media|MediaSoundComponent|SetMediaPlayer (Variables|Default|GetMediaSound) (Variables|Default|GetMedia%20Player)))

(event EventBeginPlay
  (CallFunction|PlayVideofromURL "https://www.googleapis.com/drive/v3/files/1M6BejFYSxRvaxzYZQVAI9koXle0RU98E?alt=media&key=AIzaSyDRJr38YKbwCjfi1YnDs1QvJ-PdxatecX0")
  (Utilities|FlowControl|Delay 5.0))

(fn ConstructionScript)

(fn PlayVideofromURL
  (params (NewParam :type String))
  (Variables|/Script/MediaAssets.StreamMediaSource|SetStreamUrl (Variables|Default|GetStreamMediaSource) NewParam)
  (Media|MediaPlayer|OpenSource (Variables|Default|GetMedia%20Player) (Variables|Default|GetStreamMediaSource))
  (Media|MediaSoundComponent|SetMediaPlayer (Variables|Default|GetMediaSound) (Variables|Default|GetMedia%20Player)))